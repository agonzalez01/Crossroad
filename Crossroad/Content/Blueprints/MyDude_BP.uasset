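; MyDude_BP is a character Blueprint, apparently for a Belica player character, with movement state and replay test controls.
; Tick mirrors the falling state into IsJumping, and holding right mouse halves walk speed.
; Number keys start and stop recording or play a replay through ReplayGameInstance, alongside small debug and flag hooks.
; Most other logic, including aiming, animation flags, effects, sounds and rotation, is disconnected and never runs.
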(event Custom|MovingBackw
  (params (chill :type Boolean))
  (Variables|Default|SetisChillin chill))

(event EventBeginPlay)

(event Collision|EventActorBeginOverlap
  (params (OtherActor :type Actor%20Object%20Reference)))

(event EventTick
  (params (DeltaSeconds :type Float%20%28single-precision%29))
  (Variables|Default|SetIsJumping (AI|Components|NavMovement|IsFalling (Variables|Character|GetCharacterMovement))))

(event Input|KeyboardEvents|O
  (params (Key :type Key%20Structure :default "None"))
  (:Pressed
    (Variables|Default|Setshouldchill false)))

(event Input|MouseEvents|RightMouseButton
  (params (Key :type Key%20Structure :default "None"))
  (bind _charactermovement (Variables|Character|GetCharacterMovement))
  (:Pressed
    (Variables|/Script/Engine.CharacterMovementComponent|SetMaxWalkSpeed _charactermovement 3e+02))
  (:Released
    (Variables|/Script/Engine.CharacterMovementComponent|SetMaxWalkSpeed _charactermovement 6e+02)))

(event Input|KeyboardEvents|W
  (params (Key :type Key%20Structure :default "None")))

(event Input|KeyboardEvents|Q
  (params (Key :type Key%20Structure :default "None")))

(event Input|MouseEvents|LeftMouseButton
  (params (Key :type Key%20Structure :default "None")))

(event Input|KeyboardEvents|1
  (params (Key :type Key%20Structure :default "None"))
  (:Pressed
    (bind _asreplay_game_instance (Utilities|Casting|CastToReplayGameInstance (Game|GetGameInstance)))
    (Class|ReplayGameInstance|StartRecording _asreplay_game_instance)))

(event Input|KeyboardEvents|2
  (params (Key :type Key%20Structure :default "None"))
  (:Pressed
    (bind _asreplay_game_instance (Utilities|Casting|CastToReplayGameInstance (Game|GetGameInstance)))
    (Class|ReplayGameInstance|StopRecording _asreplay_game_instance)))

(event Input|KeyboardEvents|3
  (params (Key :type Key%20Structure :default "None"))
  (:Pressed
    (bind _asreplay_game_instance (Utilities|Casting|CastToReplayGameInstance (Game|GetGameInstance)))
    (Class|ReplayGameInstance|StartReplay _asreplay_game_instance)))

(event Input|KeyboardEvents|5
  (params (Key :type Key%20Structure :default "None"))
  (:Pressed
    (Development|PrintString (Utilities|String|ToString(Boolean) (Variables|Default|GetcanMove)))))

(event Input|MouseEvents|LeftMouseButton
  (params (Key :type Key%20Structure :default "None")))

(fn ConstructionScript)

(fn SetFalse)